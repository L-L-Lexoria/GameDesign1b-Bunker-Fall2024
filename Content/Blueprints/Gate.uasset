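; Double gate actor that opens when the third-person player character enters its trigger box.
; The box overlap plays the Open timeline, which moves and rotates both gate leaves in world space.
; Each leaf follows a transform lerp between its own A and B marker components, so the markers define the closed and open poses.
; Nothing reverses the timeline to close the gate.
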(event `self.Box.OnComponentBeginOverlap`
  (params (OverlappedComponent :type "PrimitiveComponent Object Reference") (OtherActor :type "Actor Object Reference") (OtherComp :type "PrimitiveComponent Object Reference") (OtherBodyIndex :type Integer) (bFromSweep :type Boolean) (SweepResult :type "HitResult Structure (by ref)"))
  (cast `/Game/ThirdPerson/Blueprints/BP_ThirdPersonCharacter` OtherActor)
  (bind (_direction _newtrack_0) (`Timeline|Open`)
    (:`Update`
      (bind (_returnvalue_location _returnvalue_rotation) (`KismetMathLibrary.BreakTransform` (`KismetMathLibrary.TLerp` (`SceneComponent.K2_GetComponentToWorld` (`self.LeftGateA`)) (`SceneComponent.K2_GetComponentToWorld` (`self.LeftGateB`)) _newtrack_0)))
      (`SceneComponent.K2_SetWorldLocationAndRotation` (`self.Gate`) _returnvalue_location _returnvalue_rotation false false)
      (bind (_returnvalue_location_2 _returnvalue_rotation_2) (`KismetMathLibrary.BreakTransform` (`KismetMathLibrary.TLerp` (`SceneComponent.K2_GetComponentToWorld` (`self.RightGateA`)) (`SceneComponent.K2_GetComponentToWorld` (`self.RightGateB`)) _newtrack_0)))
      (`SceneComponent.K2_SetWorldLocationAndRotation` (`self.Gate1`) _returnvalue_location_2 _returnvalue_rotation_2 false false))))

(fn `UserConstructionScript`)