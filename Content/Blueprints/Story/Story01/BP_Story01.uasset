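; Story trigger actor that shows the Story01 narrative sequence when the player character enters its TriggerZone.
; It displays three story widgets in turn, each for a fixed delay, calling RemoveAllWidgets between them, which also clears any other viewport UI.
; HasBeenPlayed is set only after the last widget is removed, so re-entering mid-sequence is not blocked.
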(event `self.TriggerZone.OnComponentBeginOverlap`
  (params (OverlappedComponent :type "PrimitiveComponent Object Reference") (OtherActor :type "Actor Object Reference") (OtherComp :type "PrimitiveComponent Object Reference") (OtherBodyIndex :type Integer) (bFromSweep :type Boolean) (SweepResult :type "HitResult Structure (by ref)"))
  (if (not (`self.HasBeenPlayed`))
    (cast `/Game/ThirdPerson/Blueprints/BP_ThirdPersonCharacter` OtherActor)
    (bind _returnvalue (`|CreateWidget` "/Game/Blueprints/Story/Story01/W_Story01_0.W_Story01_0_C"))
    (`UserWidget.AddToViewport` _returnvalue 0)
    (`KismetSystemLibrary.Delay` 3.0)
    (`WidgetLayoutLibrary.RemoveAllWidgets`)
    (bind _returnvalue_2 (`|CreateWidget` "/Game/Blueprints/Story/Story01/W_Story01_1.W_Story01_1_C"))
    (`UserWidget.AddToViewport` _returnvalue_2 0)
    (`KismetSystemLibrary.Delay` 5.0)
    (`WidgetLayoutLibrary.RemoveAllWidgets`)
    (bind _returnvalue_3 (`|CreateWidget` "/Game/Blueprints/Story/Story01/W_Story01_2.W_Story01_2_C"))
    (`UserWidget.AddToViewport` _returnvalue_3 0)
    (`KismetSystemLibrary.Delay` 3.0)
    (`WidgetLayoutLibrary.RemoveAllWidgets`)
    (set `self.HasBeenPlayed` true)))

(fn `UserConstructionScript`)