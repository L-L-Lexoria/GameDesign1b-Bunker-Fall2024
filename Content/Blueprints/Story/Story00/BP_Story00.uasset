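; BP_Story00 is an actor that plays the Story00 sequence as timed fullscreen widgets when play begins.
; BeginPlay creates the W_Story00_0, W_Story00_1 and W_Story00_2 widgets in turn for player 0, separated by fixed delays of a few seconds.
; Each step clears every widget from the viewport with RemoveAllWidgets, so any other on-screen UI is removed too.
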(event `self.ReceiveBeginPlay`
  (bind _returnvalue (`GameplayStatics.GetPlayerController` 0))
  (bind _returnvalue_2 (`|CreateWidget` "/Game/Blueprints/Story/Story00/W_Story00_0.W_Story00_0_C" _returnvalue))
  (`UserWidget.AddToViewport` _returnvalue_2 0)
  (`KismetSystemLibrary.Delay` 3.0)
  (`WidgetLayoutLibrary.RemoveAllWidgets`)
  (bind _returnvalue_3 (`|CreateWidget` "/Game/Blueprints/Story/Story00/W_Story00_1.W_Story00_1_C" _returnvalue))
  (`UserWidget.AddToViewport` _returnvalue_3 0)
  (`KismetSystemLibrary.Delay` 5.0)
  (`WidgetLayoutLibrary.RemoveAllWidgets`)
  (bind _returnvalue_4 (`|CreateWidget` "/Game/Blueprints/Story/Story00/W_Story00_2.W_Story00_2_C" _returnvalue))
  (`UserWidget.AddToViewport` _returnvalue_4 0)
  (`KismetSystemLibrary.Delay` 3.0)
  (`WidgetLayoutLibrary.RemoveAllWidgets`))

(fn `UserConstructionScript`)